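; SolarDefaultCharacter is a character Blueprint that shows a player interface and exposes the character's current health.
; On BeginPlay, non-dedicated-server instances call ShowUI, which creates the Interface widget and adds it to the viewport only where the character lacks authority.
; GetCurrentHP returns the current HP value from the CharacterVitals data.
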(event `self.ReceiveBeginPlay`
  (if (not (`KismetSystemLibrary.IsDedicatedServer` null))
    (`self.ShowUI`)))

(fn `Get Current HP`
  (returns (fHP :type "Float (double-precision)"))
  (return (`.fCurrentHP` (break `Vitals` (`self.characterVitals`)))))

(fn `ShowUI`
  (if (not (`self.HasAuthority`))
    (bind _returnvalue (`WidgetBlueprintLibrary.Create` null "/Game/UI/Interface.Interface_C"))
    (`UserWidget.AddToViewport` _returnvalue 0)))

(fn `UserConstructionScript`)